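; BP_StatComp is a stat component that tracks its owner's health and timed casting state, with RepNotify functions for replication.
; Damage flows through a clamped SetHp, which broadcasts health changes and signals when HP reaches zero.
; Casting records the server world start time and runs a timer that signals success unless cancelled.
; OnRep handlers rebroadcast current HP and casting state to listeners.
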(event Custom|Server_CancleCast
  (Variables|Default|SetIsCasting false)
  (Utilities|Time|ClearandInvalidateTimerbyHandle (Variables|Default|GetCastingTimerHandle))
  (Default|CallOnCastingStateChange (Variables|Default|GetCastingDuration) false (Variables|Default|GetCastStartServerTime)))

(event Custom|Server_BeginCast
  (params (InDuration :type Float%20%28double-precision%29))
  (Variables|Default|SetIsCasting true)
  (Variables|Default|SetCastingDuration InDuration)
  (bind _output_get (Variables|Default|SetCastStartServerTime (GameState|GetServerWorldTimeSeconds (Game|GetGameState))))
  (Utilities|Time|ClearandInvalidateTimerbyHandle (Variables|Default|GetCastingTimerHandle))
  (bind _returnvalue (Utilities|Time|SetTimerbyFunctionName 0 "FinishCast_Internal" (Variables|Default|GetCastingDuration)))
  (Variables|Default|SetCastingTimerHandle _returnvalue)
  (Default|CallOnCastingStateChange (Variables|Default|GetCastingDuration) true _output_get))

(event EventBeginPlay)

(event EventTick
  (params (DeltaSeconds :type Float%20%28single-precision%29)))

(fn GetCurrentHp
  (return (Variables|Default|GetCurrentHp)))

(fn GetMaxHp
  (return (Variables|Default|GetMaxHp)))

(fn ApplyDamage
  (params (InDamage :type Float%20%28double-precision%29))
  (LocalVariables|SetPrevHp (Variables|Default|GetCurrentHp))
  (LocalVariables|SetActualDamage (Math|Float|Clamp(Float) InDamage 0.0 InDamage))
  (CallFunction|SetHp (- (LocalVariables|GetPrevHp) (LocalVariables|GetActualDamage))))

(fn SetHp
  (params (NewHp :type Float%20%28double-precision%29))
  (bind _output_get (Variables|Default|SetCurrentHp (Math|Float|Clamp(Float) NewHp 0.0 (Variables|Default|GetMaxHp))))
  (Default|CallOnHealthChangeDelegate _output_get (Variables|Default|GetMaxHp))
  (if (<= _output_get 0.0)
    (Default|CallOnHpZero)))

(fn OnRepCurrentHp
  (Default|CallOnHealthChangeDelegate (Variables|Default|GetCurrentHp) (Variables|Default|GetMaxHp)))

(fn OnRepMaxHp)

(fn OnRepIsCasting
  (Default|CallOnCastingStateChange (Variables|Default|GetCastingDuration) (Variables|Default|GetIsCasting) (Variables|Default|GetCastStartServerTime)))

(fn FinishCastInternal
  (Variables|Default|SetIsCasting false)
  (Utilities|Time|ClearandInvalidateTimerbyHandle (Variables|Default|GetCastingTimerHandle))
  (Default|CallOnCastingSuccededDelegate))